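; BP_Toggleable_Component is an actor component that holds a replicated on/off state for its owner.
; Toggle writes IsOn, and its OnRep broadcasts the NotifyToggleableUpdate dispatcher so listeners can react to the change.
; It caches the owning actor on BeginPlay and declares AsToggleableComponent accessors, whose bodies are empty returns.
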(event EventToggle
  (params (NewToggle :type Boolean))
  (Variables|ToggleableComponent|SetIsOn NewToggle))

(event EventBeginPlay
  (Variables|ToggleableComponent|SetOwner (Components|GetOwner)))

(fn OnRepIson
  (Default|CallNotifyToggleableUpdate (Variables|ToggleableComponent|GetIsOn)))

(fn AsToggleableComponent
  (return 0))

(fn AsToggleableComponentObject
  (return 0))