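; Actor component that drives data-driven events and interactions by adding behaviour components to actors at runtime.
; BeginPlay, EndPlay, damage and interactions each spawn an EventComponent on the owner for every matching Events entry.
; Interactions also update, add or remove owner components like toggle, gate, sound and weapon.
; DoEnvironmentManagement applies interaction, visibility and transform components to actors chosen by reference, class or tag, and adds spawners to the owner.
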(event Custom|EndPlayTrigger
  (params (Actor :type Actor%20Object%20Reference) (EndPlayReason :type EEndPlayReason%20Enum :default "Destroyed"))
  (CallFunction|DoAllEventsbyType "NewEnumerator1"))

(event Custom|DamageTrigger
  (params (DamagedActor :type Actor%20Object%20Reference) (Damage :type Float%20%28single-precision%29) (DamageType :type Damage%20Type%20Object%20Reference) (InstigatedBy :type Controller%20Object%20Reference) (DamageCauser :type Actor%20Object%20Reference))
  (CallFunction|DoAllEventsbyType "NewEnumerator2"))

(event EventBeginPlay
  (Variables|EventControllerComponent|SetOwner (Components|GetOwner))
  (Utilities|FlowControl|Sequence
    (:then_0
      (Game|BindEventtoOnEndPlay (Variables|EventControllerComponent|GetOwner) (delegate Custom|EndPlayTrigger))
      (EventDispatchers|BindEventtoOnTakeAnyDamage (Variables|EventControllerComponent|GetOwner) (delegate Custom|DamageTrigger)))
    (:then_1
      (CallFunction|DoAllEventsbyType "NewEnumerator0"))))

(fn GetEventsbyType
  (params (EventType :type E_EventType%20Enum :default "NewEnumerator0"))
  (for _array_element (Variables|EventControllerComponent|GetEvents)
    (if (Utilities|Enum|Equal(Enum) EventType (.EventType (Utilities|Struct|BreakS_Event _array_element)))
      (Utilities|Array|Add (LocalVariables|GetLocalEventDataArray) _array_element)))
  (return (LocalVariables|GetLocalEventDataArray)))

(fn DoAllEventsbyType
  (params (EventType :type E_EventType%20Enum :default "NewEnumerator0"))
  (LocalVariables|SetLocalEventArray (CallFunction|GetEventsbyType EventType))
  (for _array_element (LocalVariables|GetLocalEventArray)
    (LocalVariables|SetLocalCurrentEvent _array_element)
    (Game|AddComponentbyClass (Variables|EventControllerComponent|GetOwner) (Variables|EventControllerComponentConstants|GetEventComponent) (LocalVariables|GetLocalCurrentEvent))))

(fn DoEnvironmentManagement
  (params (EventData :type S%20Event%20Data%20Structure%20%28by%20ref%29))
  (bind _environment (Utilities|Struct|BreakS_EventData EventData))
  (bind (_actorinteraction _actorvisibility _actortransform _actorspawn) (Utilities|Struct|BreakS_EventEnvironmentData _environment))
  (Utilities|FlowControl|Sequence
    (:then_0
      (for _array_element _actorinteraction
        (for _array_element_2 (.ActorData (Utilities|Struct|BreakS_EnvironmentActorInteractionData _array_element))
          (Utilities|FlowControl|Sequence
            (:then_0
              (CallFunction|AddInteractComponenttoActors (.ManagedActors (Utilities|Struct|BreakS_ManagedActors _array_element_2)) (.InteractionData (Utilities|Struct|BreakS_EnvironmentActorInteractionData _array_element))))
            (:then_1
              (bind _outactors (Utilities|ForEachActorfromClass (.ManagedActorsByClass (Utilities|Struct|BreakS_ManagedActors _array_element_2))))
              (CallFunction|AddInteractComponenttoActors _outactors (.InteractionData (Utilities|Struct|BreakS_EnvironmentActorInteractionData _array_element))))
            (:then_2
              (bind _outactors_2 (Utilities|ForEachActorfromTag (.ManagedActorsByTag (Utilities|Struct|BreakS_ManagedActors _array_element_2))))
              (CallFunction|AddInteractComponenttoActors _outactors_2 (.InteractionData (Utilities|Struct|BreakS_EnvironmentActorInteractionData _array_element))))))))
    (:then_1
      (for _array_element_3 _actorvisibility
        (Utilities|FlowControl|Sequence
          (:then_0
            (CallFunction|AddVisiblityComponenttoActors (.ManagedActors (Utilities|Struct|BreakS_ManagedActors (.Managed (Utilities|Struct|BreakS_EnvironmentActorVisibilityData _array_element_3)))) (.VisibilityData (Utilities|Struct|BreakS_EnvironmentActorVisibilityData _array_element_3))))
          (:then_1
            (bind _outactors_3 (Utilities|ForEachActorfromClass (.ManagedActorsByClass (Utilities|Struct|BreakS_ManagedActors (.Managed (Utilities|Struct|BreakS_EnvironmentActorVisibilityData _array_element_3))))))
            (CallFunction|AddVisiblityComponenttoActors _outactors_3 (.VisibilityData (Utilities|Struct|BreakS_EnvironmentActorVisibilityData _array_element_3))))
          (:then_2
            (bind _outactors_4 (Utilities|ForEachActorfromTag (.ManagedActorsByTag (Utilities|Struct|BreakS_ManagedActors (.Managed (Utilities|Struct|BreakS_EnvironmentActorVisibilityData _array_element_3))))))
            (CallFunction|AddVisiblityComponenttoActors _outactors_4 (.VisibilityData (Utilities|Struct|BreakS_EnvironmentActorVisibilityData _array_element_3)))))))
    (:then_2
      (for _array_element_4 _actortransform
        (Utilities|FlowControl|Sequence
          (:then_0
            (CallFunction|AddTransformComponenttoActors (.ManagedActors (Utilities|Struct|BreakS_ManagedActors (.Managed (Utilities|Struct|BreakS_EnvironmentActorTransformData _array_element_4)))) (.TransformData (Utilities|Struct|BreakS_EnvironmentActorTransformData _array_element_4))))
          (:then_1
            (bind _outactors_5 (Utilities|ForEachActorfromClass (.ManagedActorsByClass (Utilities|Struct|BreakS_ManagedActors (.Managed (Utilities|Struct|BreakS_EnvironmentActorTransformData _array_element_4))))))
            (CallFunction|AddTransformComponenttoActors _outactors_5 (.TransformData (Utilities|Struct|BreakS_EnvironmentActorTransformData _array_element_4))))
          (:then_2
            (bind _outactors_6 (Utilities|ForEachActorfromTag (.ManagedActorsByTag (Utilities|Struct|BreakS_ManagedActors (.Managed (Utilities|Struct|BreakS_EnvironmentActorTransformData _array_element_4))))))
            (CallFunction|AddTransformComponenttoActors _outactors_6 (.TransformData (Utilities|Struct|BreakS_EnvironmentActorTransformData _array_element_4)))))))
    (:then_3
      (for _array_element_5 _actorspawn
        (bind _returnvalue (Game|AddComponentbyClass (Variables|EventControllerComponent|GetOwner) (Variables|EventControllerComponentConstants|GetSpawnerComponent) _array_element_5))
        (Default|CallNotifySpawnerComponentAdded _returnvalue)))))

(fn DoInteraction
  (params (InteractComponent :type BP%20Interact%20Component%20Object%20Reference))
  (bind _output_get (LocalVariables|SetLocalInteractComponent InteractComponent))
  (switch Utilities|FlowControl|Switch|SwitchonE_EventType (Variables|/Game/Project4/Blueprints/Component/EventController/BP_InteractComponent.BP_InteractComponent_C|GetEvent%20Type _output_get)
    (:NewEnumerator3
      (CallFunction|UpdateorAddToggleComponent true))
    (:NewEnumerator4
      (CallFunction|UpdateorAddToggleComponent false))
    (:NewEnumerator21
      (CallFunction|UpdateorAddAccessComponent true))
    (:NewEnumerator22
      (CallFunction|UpdateorAddAccessComponent false))
    (:NewEnumerator5
      (CallFunction|UpdateorAddAlarmComponent true))
    (:NewEnumerator6
      (CallFunction|UpdateorAddAlarmComponent false))
    (:NewEnumerator23
      (CallFunction|UpdateorAddGateComponent true))
    (:NewEnumerator24
      (CallFunction|UpdateorAddGateComponent false))
    (:NewEnumerator7
      (CallFunction|UpdateorAddTargetingComponent true (LocalVariables|GetLocalInteractComponent)))
    (:NewEnumerator8
      (CallFunction|UpdateorAddTargetingComponent false (LocalVariables|GetLocalInteractComponent)))
    (:NewEnumerator25
      (CallFunction|UpdateorAddHoverComponent true (LocalVariables|GetLocalInteractComponent)))
    (:NewEnumerator27
      (CallFunction|UpdateorAddHoverComponent false (LocalVariables|GetLocalInteractComponent)))
    (:NewEnumerator28
      (CallFunction|AddTeleportComponenttoActor (LocalVariables|GetLocalInteractComponent)))
    (:NewEnumerator9
      (CallFunction|AddorRemoveHealthComponent true))
    (:NewEnumerator10
      (CallFunction|AddorRemoveHealthComponent false))
    (:NewEnumerator29
      (CallFunction|UpdateorAddSoundComponent true (LocalVariables|GetLocalInteractComponent)))
    (:NewEnumerator30
      (CallFunction|UpdateorAddSoundComponent false (LocalVariables|GetLocalInteractComponent)))
    (:NewEnumerator31
      (CallFunction|AddorRemoveWeaponComponent true (LocalVariables|GetLocalInteractComponent)))
    (:NewEnumerator32
      (CallFunction|AddorRemoveWeaponComponent false (LocalVariables|GetLocalInteractComponent)))
    (:NewEnumerator33
      (CallFunction|UpdateorAddNiagaraEffectComponent true (LocalVariables|GetLocalInteractComponent)))
    (:NewEnumerator34
      (CallFunction|UpdateorAddNiagaraEffectComponent false (LocalVariables|GetLocalInteractComponent)))
    (:NewEnumerator35
      (CallFunction|UpdateorAddCounterComponent false false))
    (:NewEnumerator36
      (CallFunction|UpdateorAddCounterComponent true true))
    (:NewEnumerator37
      (CallFunction|UpdateorAddCounterComponent true false))))

(fn AddVisiblityComponenttoActors
  (params (Actors :type Array%20of%20Actor%20Object%20References) (VisibilityData :type S%20Visibility%20Data%20Structure))
  (for _array_element Actors
    (bind _returnvalue (Game|AddComponentbyClass _array_element (Variables|EventControllerComponentConstants|GetVisibilityComponent) VisibilityData))
    (Default|CallNotifyVisibilityCompAdded _returnvalue)))

(fn AddTransformComponenttoActors
  (params (Actors :type Array%20of%20Actor%20Object%20References) (TransformData :type S%20Transform%20Data%20Structure))
  (for _array_element Actors
    (bind _returnvalue (Game|AddComponentbyClass _array_element (Variables|EventControllerComponentConstants|GetTransformComponent) TransformData))
    (Default|CallNotifyTransformCompAdded _returnvalue)))

(fn AddInteractComponenttoActors
  (params (Actors :type Array%20of%20Actor%20Object%20References) (InteractionData :type Array%20of%20S%20Interaction%20Data%20Structures))
  (LocalVariables|SetLocalInteractionDataArray InteractionData)
  (for _array_element Actors
    (LocalVariables|SetLocalCurrentActor _array_element)
    (for _array_element_2 (LocalVariables|GetLocalInteractionDataArray)
      (LocalVariables|SetLocalCurrentInteractionData _array_element_2)
      (Utilities|FlowControl|Sequence
        (:then_0
          (bind _returnvalue (Game|AddComponentbyClass (LocalVariables|GetLocalCurrentActor) (Variables|EventControllerComponentConstants|GetInteractionComponent) (Variables|EventControllerComponent|GetOwner) (LocalVariables|GetLocalCurrentInteractionData)))
          (LocalVariables|SetLocalInteractionComponent _returnvalue))
        (:then_1
          (Default|CallNotifyInteractCompAdded (LocalVariables|GetLocalInteractionComponent)))))))

(fn AddTeleportComponenttoActor
  (params (InteractComponent :type BP%20Interact%20Component%20Object%20Reference))
  (bind _defaultteleporttoactor (Variables|/Game/Project4/Blueprints/Component/EventController/BP_InteractComponent.BP_InteractComponent_C|GetDefaultTeleportToActor InteractComponent))
  (LocalVariables|SetLocalTeleportLocation (Variables|/Game/Project4/Blueprints/Component/EventController/BP_InteractComponent.BP_InteractComponent_C|GetDefaultTeleportToLocation InteractComponent))
  (Utilities|IsValid _defaultteleporttoactor
    (:Is%20Valid
      (LocalVariables|SetLocalTeleportLocation (Transformation|GetActorLocation _defaultteleporttoactor)))
    (:Is%20Not%20Valid
      _))
  (bind _returnvalue (Game|AddComponentbyClass (Variables|EventControllerComponent|GetOwner) (Variables|EventControllerComponentConstants|GetTeleportComponent) (LocalVariables|GetLocalTeleportLocation)))
  (Default|CallNotifyTeleportComponentAdded _returnvalue))

(fn UpdateorAddToggleComponent
  (params (NewToggle :type Boolean))
  (bind _toggleablecomponent (Variables|EventControllerComponentConstants|GetToggleableComponent))
  ;[1 1 1] update or add toggle comp
  (bind _returnvalue (Utilities|GetValidComponentbyClass _toggleablecomponent)
    (:Is%20Valid
      (Class|BPIToggle|Toggle(Message) _returnvalue NewToggle))
    (:Is%20Not%20Valid
      (bind _returnvalue_2 (Game|AddComponentbyClass (Variables|EventControllerComponent|GetOwner) _toggleablecomponent NewToggle))
      (Default|CallNotifyToggleCompAdded _returnvalue_2))))

(fn UpdateorAddAlarmComponent
  (params (NewAlarm :type Boolean))
  (bind _alarmcomponent (Variables|EventControllerComponentConstants|GetAlarmComponent))
  ;[1 1 1] Update or add alarm comp
  (bind _returnvalue (Utilities|GetValidComponentbyClass _alarmcomponent)
    (:Is%20Valid
      (Class|BPIToggle|Toggle(Message) _returnvalue NewAlarm))
    (:Is%20Not%20Valid
      (bind _returnvalue_2 (Game|AddComponentbyClass (Variables|EventControllerComponent|GetOwner) _alarmcomponent NewAlarm))
      (Default|CallNotifyAlarmCompAdded _returnvalue_2))))

(fn UpdateorAddTargetingComponent
  (params (IsTargeting :type Boolean) (InteractComponent :type BP%20Interact%20Component%20Object%20Reference))
  (bind _targetingcomponent (Variables|EventControllerComponentConstants|GetTargetingComponent))
  ;[1 1 1] Update or add targeting comp
  (bind _returnvalue (Utilities|GetValidComponentbyClass _targetingcomponent)
    (:Is%20Valid
      (Class|BPIToggle|Toggle(Message) _returnvalue IsTargeting))
    (:Is%20Not%20Valid
      (bind _returnvalue_2 (Game|AddComponentbyClass (Variables|EventControllerComponent|GetOwner) _targetingcomponent IsTargeting (Variables|/Game/Project4/Blueprints/Component/EventController/BP_InteractComponent.BP_InteractComponent_C|GetDefaultTargetingAxisXorY InteractComponent) (Variables|/Game/Project4/Blueprints/Component/EventController/BP_InteractComponent.BP_InteractComponent_C|GetDefaultTargetActor InteractComponent) (Variables|/Game/Project4/Blueprints/Component/EventController/BP_InteractComponent.BP_InteractComponent_C|GetDefault%20Target%20Location InteractComponent) (Variables|/Game/Project4/Blueprints/Component/EventController/BP_InteractComponent.BP_InteractComponent_C|GetInterp%20Speed InteractComponent)))
      (Default|CallNotifyTargetingCompAdded _returnvalue_2))))

(fn UpdateorAddAccessComponent
  (params (IsLocked :type Boolean))
  (bind _accesscomponent (Variables|EventControllerComponentConstants|GetAccessComponent))
  ;[1 1 1] update or add toggle comp
  (bind _returnvalue (Utilities|GetValidComponentbyClass _accesscomponent)
    (:Is%20Valid
      (Class|BPIToggle|Toggle(Message) _returnvalue IsLocked))
    (:Is%20Not%20Valid
      (bind _returnvalue_2 (Game|AddComponentbyClass (Variables|EventControllerComponent|GetOwner) _accesscomponent IsLocked))
      (Default|CallNotifyAccessComponentAdded _returnvalue_2))))

(fn UpdateorAddGateComponent
  (params (IsOpen :type Boolean))
  (bind _gatecomponent (Variables|EventControllerComponentConstants|GetGateComponent))
  ;[1 1 1] update or add toggle comp
  (bind _returnvalue (Utilities|GetValidComponentbyClass _gatecomponent)
    (:Is%20Valid
      (Class|BPIToggle|Toggle(Message) _returnvalue IsOpen))
    (:Is%20Not%20Valid
      (bind _returnvalue_2 (Game|AddComponentbyClass (Variables|EventControllerComponent|GetOwner) _gatecomponent IsOpen))
      (Default|CallNotifyGateComponentAdded _returnvalue_2))))

(fn UpdateorAddHoverComponent
  (params (IsHover :type Boolean) (InteractComponent :type BP%20Interact%20Component%20Object%20Reference))
  (bind _hovercomponent (Variables|EventControllerComponentConstants|GetHoverComponent))
  ;[1 1 1] update or add toggle comp
  (bind _returnvalue (Utilities|GetValidComponentbyClass _hovercomponent)
    (:Is%20Valid
      (Class|BPIToggle|Toggle(Message) _returnvalue IsHover))
    (:Is%20Not%20Valid
      (bind _returnvalue_2 (Game|AddComponentbyClass (Variables|EventControllerComponent|GetOwner) _hovercomponent IsHover (Variables|/Game/Project4/Blueprints/Component/EventController/BP_InteractComponent.BP_InteractComponent_C|GetDefault%20Hover%20Vector InteractComponent) (Variables|/Game/Project4/Blueprints/Component/EventController/BP_InteractComponent.BP_InteractComponent_C|GetInterp%20Speed InteractComponent)))
      (Default|CallNotifyHoverComponentAdded _returnvalue_2))))

(fn UpdateorAddSoundComponent
  (params (IsSoundOn :type Boolean) (InteractComponent :type BP%20Interact%20Component%20Object%20Reference))
  (bind _soundcomponent (Variables|EventControllerComponentConstants|GetSoundComponent))
  ;[1 1 1] update or add toggle comp
  (bind _returnvalue (Utilities|GetValidComponentbyClass _soundcomponent)
    (:Is%20Valid
      (Class|BPIToggle|Toggle(Message) _returnvalue IsSoundOn))
    (:Is%20Not%20Valid
      (bind _returnvalue_2 (Game|AddComponentbyClass :self (Variables|EventControllerComponent|GetOwner) :Class _soundcomponent :IsSoundOn IsSoundOn :Sound2D (Variables|/Game/Project4/Blueprints/Component/EventController/BP_InteractComponent.BP_InteractComponent_C|GetDefault%20Sound%202D InteractComponent) :Sound3D (Variables|/Game/Project4/Blueprints/Component/EventController/BP_InteractComponent.BP_InteractComponent_C|GetDefault%20Sound%203D InteractComponent) :SoundAttenuation (Variables|/Game/Project4/Blueprints/Component/EventController/BP_InteractComponent.BP_InteractComponent_C|GetDefault%20Sound%20Attenuation InteractComponent)))
      (Default|CallNotifySoundComponentAdded _returnvalue_2))))

(fn UpdateorAddNiagaraEffectComponent
  (params (IsEffectOn :type Boolean) (InteractComponent :type BP%20Interact%20Component%20Object%20Reference))
  (bind _niagaraeffectcomponent (Variables|EventControllerComponentConstants|GetNiagaraEffectComponent))
  ;[1 1 1] update or add toggle comp
  (bind _returnvalue (Utilities|GetValidComponentbyClass _niagaraeffectcomponent)
    (:Is%20Valid
      (Class|BPIToggle|Toggle(Message) _returnvalue IsEffectOn))
    (:Is%20Not%20Valid
      (bind _returnvalue_2 (Game|AddComponentbyClass (Variables|EventControllerComponent|GetOwner) _niagaraeffectcomponent false))
      (Utilities|FlowControl|Sequence
        (:then_0
          (Default|CallNotifyNiagaraEffectComponentAdded _returnvalue_2))
        (:then_1
          (Class|NiagaraComponent|SetAsset _returnvalue_2 (Variables|/Game/Project4/Blueprints/Component/EventController/BP_InteractComponent.BP_InteractComponent_C|GetDefaultNiagaraSystem InteractComponent) true))))))

(fn UpdateorAddCounterComponent
  (params (ShouldModify :type Boolean) (Increment :type Boolean))
  (bind _countercomponent (Variables|EventControllerComponentConstants|GetCounterComponent))
  ;[1 1 1] update or add toggle comp
  (Utilities|FlowControl|Sequence
    (:then_0
      (bind _returnvalue (Utilities|GetValidComponentbyClass _countercomponent)
        (:Is%20Valid
          (LocalVariables|SetLocalCounterComponent _returnvalue))
        (:Is%20Not%20Valid
          (bind _returnvalue_2 (Game|AddComponentbyClass (Variables|EventControllerComponent|GetOwner) _countercomponent 0))
          (LocalVariables|SetLocalCounterComponent _returnvalue_2))))
    (:then_1
      (if ShouldModify
        (if Increment
          (Class|BPICounter|IncrementCounter(Message) (LocalVariables|GetLocalCounterComponent))
          (else
            (Class|BPICounter|DecrementCounter(Message) (LocalVariables|GetLocalCounterComponent))))))
    (:then_2
      (bind _countercomponent_2 (Class|BPICounter|AsCounterComponent(Message) (LocalVariables|GetLocalCounterComponent)))
      (Default|CallNotifyCounterComponentAdded _countercomponent_2))))

(fn AddorRemoveHealthComponent
  (params (IsAdding :type Boolean))
  ;[1 1 1] health comp
  (Utilities|FlowControl|Sequence
    (:then_0
      (bind _returnvalue (Utilities|GetValidComponentbyClass (Variables|EventControllerComponentConstants|GetHealthComponent))
        (:Is%20Valid
          (Components|DestroyComponent _returnvalue))))
    (:then_1
      (if IsAdding
        (bind _returnvalue_2 (Game|AddComponentbyClass (Variables|EventControllerComponent|GetOwner) (Variables|EventControllerComponentConstants|GetHealthComponent)))
        (Default|CallNotifyHealthComponentAdded _returnvalue_2)))))

(fn AddorRemoveWeaponComponent
  (params (IsAdding :type Boolean) (InteractComponent :type BP%20Interact%20Component%20Object%20Reference))
  ;[1 1 1] health comp
  (Utilities|FlowControl|Sequence
    (:then_0
      (bind _returnvalue (Utilities|GetValidComponentbyClass (Variables|EventControllerComponentConstants|GetWeaponComponent))
        (:Is%20Valid
          (Components|DestroyComponent _returnvalue))))
    (:then_1
      (if IsAdding
        (bind _returnvalue_2 (Game|AddComponentbyClass :self (Variables|EventControllerComponent|GetOwner) :Class (Variables|EventControllerComponentConstants|GetWeaponComponent) :IsEquipped true :ProjectileClass (Variables|/Game/Project4/Blueprints/Component/EventController/BP_InteractComponent.BP_InteractComponent_C|GetDefault%20Projectile%20Class InteractComponent) :SpawnSocket (Variables|/Game/Project4/Blueprints/Component/EventController/BP_InteractComponent.BP_InteractComponent_C|GetDefaultProjectileSocket InteractComponent) :Sound3D (Variables|/Game/Project4/Blueprints/Component/EventController/BP_InteractComponent.BP_InteractComponent_C|GetDefault%20Sound%203D InteractComponent) :SoundAttenuation (Variables|/Game/Project4/Blueprints/Component/EventController/BP_InteractComponent.BP_InteractComponent_C|GetDefault%20Sound%20Attenuation InteractComponent)))
        (Utilities|FlowControl|Sequence
          (:then_0
            (Components|SkeletalMesh|SetSkeletalMeshAsset _returnvalue_2 (Variables|/Game/Project4/Blueprints/Component/EventController/BP_InteractComponent.BP_InteractComponent_C|GetDefaultSkeletalMesh InteractComponent)))
          (:then_1
            (Default|CallNotifyWeaponComponentAdded _returnvalue_2)))))))

(fn AsEventControllerComponent
  (return self))

(fn EventControllerInteract
  (params (ActorInteractComponent :type BP%20Interact%20Component%20Object%20Reference))
  (LocalVariables|SetLocalActorInteractComp ActorInteractComponent)
  (Utilities|FlowControl|Sequence
    (:then_0
      (CallFunction|DoInteraction (LocalVariables|GetLocalActorInteractComp)))
    (:then_1
      (CallFunction|DoAllEventsbyType (Variables|/Game/Project4/Blueprints/Component/EventController/BP_InteractComponent.BP_InteractComponent_C|GetEvent%20Type (LocalVariables|GetLocalActorInteractComp))))
    (:then_2
      (return true))))