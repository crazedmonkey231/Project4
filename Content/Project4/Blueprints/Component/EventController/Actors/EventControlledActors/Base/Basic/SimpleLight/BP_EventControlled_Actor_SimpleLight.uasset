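; Base light actor driven by the event controller system, showing or hiding its Lights component based on a toggle component's state.
; On BeginPlay it listens for a toggle component being added to its event controller component, then subscribes to that toggle's updates.
; The initial state and every later toggle change set Lights hidden in game, propagated to its child components.
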(event Custom|OnToggleComponent
  (params (ToggleComponent :type BP%20Toggleable%20Component%20Object%20Reference))
  (bind _output_get (Variables|Default|SetToggle%20Component ToggleComponent))
  (EventDispatchers|BindEventtoNotifyToggleableUpdate _output_get (delegate Custom|ToggleComponentUpdate))
  (Development|SetHiddeninGame (Variables|Default|GetLights) (not (Variables|/Game/Project4/Blueprints/Component/EventController/Events/Environment/BP_Toggleable_Component.BP_Toggleable_Component_C|GetIsOn _output_get)) true))

(event Custom|ToggleComponentUpdate
  (params (CurrentToggle :type Boolean))
  (Development|SetHiddeninGame (Variables|Default|GetLights) (not CurrentToggle) true))

(event EventBeginPlay
  (EventDispatchers|BindEventtoNotifyToggleCompAdded (Variables|Default|GetBP_EventController_Component) (delegate Custom|OnToggleComponent)))

(fn ConstructionScript
  (|CallParentFunction))