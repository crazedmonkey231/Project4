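; BP_CollisionHandlerComponent is an actor component that turns overlaps on an event-controlled trigger into event controller calls.
; On BeginPlay it queries its owner through an interface message for the event-controlled object and collision list, printing an error if that object is invalid.
; It binds begin and end overlap on every collision, each firing all controller events of its own type without filtering the other actor.
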(event Custom|OnOverlap
  (params (OverlappedComponent :type Primitive%20Component%20Object%20Reference) (OtherActor :type Actor%20Object%20Reference) (OtherComp :type Primitive%20Component%20Object%20Reference) (OtherBodyIndex :type Integer) (bFromSweep :type Boolean) (SweepResult :type Hit%20Result%20Structure%20%28by%20ref%29))
  (Default|DoAllEventsbyType (Variables|/Game/Project4/Blueprints/Component/EventController/Actors/EventControlledActors/Base/BPA_EventControlled_Actor.BPA_EventControlled_Actor_C|GetBP_EventController_Component (Variables|Default|GetOwner)) "NewEnumerator11"))

(event Custom|OnEndOverlap
  (params (OverlappedComponent :type Primitive%20Component%20Object%20Reference) (OtherActor :type Actor%20Object%20Reference) (OtherComp :type Primitive%20Component%20Object%20Reference) (OtherBodyIndex :type Integer))
  (Default|DoAllEventsbyType (Variables|/Game/Project4/Blueprints/Component/EventController/Actors/EventControlledActors/Base/BPA_EventControlled_Actor.BPA_EventControlled_Actor_C|GetBP_EventController_Component (Variables|Default|GetOwner)) "NewEnumerator12"))

(event EventBeginPlay
  (bind (_eventcontrolled _collisions) (Utilities|IsValidTrigger (Components|GetOwner))
    (:Is%20Valid
      (Variables|Default|SetOwner _eventcontrolled)
      (for _array_element _collisions
        (Collision|BindEventtoOnComponentBeginOverlap _array_element (delegate Custom|OnOverlap))
        (Collision|BindEventtoOnComponentEndOverlap _array_element (delegate Custom|OnEndOverlap))))
    (:Is%20Not%20Valid
      (Development|PrintString "Invalid owner, owner must be event controlled trigger"))))