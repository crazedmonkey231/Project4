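; BP_EventController_Weapon is an event controller actor for weapons that captures references to targeting and weapon components as they are added.
; On BeginPlay it runs the parent logic, then binds to the targeting-added and weapon-added notifications of its event controller component.
; Each callback stores the received component in a variable; the graph contains no other weapon behavior, and construction only calls the parent.
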(event Custom|OnTargetingComponentAdded
  (params (TargetingComponent :type BP%20Targeting%20Component%20Object%20Reference))
  (Variables|Default|SetTargeting%20Component TargetingComponent))

(event Custom|OnWeaponComponentAdded
  (params (WeaponComponent :type BP%20Basic%20Weapon%20Component%20Object%20Reference))
  (Variables|Default|SetWeapon%20Component WeaponComponent))

(event EventBeginPlay
  (|CallParentFunction)
  (EventDispatchers|BindEventtoNotifyTargetingCompAdded (Variables|Default|GetBP_EventController_Component) (delegate Custom|OnTargetingComponentAdded))
  (EventDispatchers|BindEventtoNotifyWeaponComponentAdded (Variables|Default|GetBP_EventController_Component) (delegate Custom|OnWeaponComponentAdded)))

(fn ConstructionScript
  (|CallParentFunction))