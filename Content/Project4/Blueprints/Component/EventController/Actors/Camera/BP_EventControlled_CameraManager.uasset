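; Event-driven camera manager that handles target lock-on for its owning player controller.
; It binds to its event controller component to receive the targeting component, then follows that component's targeting-active notifications.
; While targeting is active, look input is ignored and a looping timer, rather than Tick, interpolates control rotation toward the component's target rotation.
; The timer is cleared when targeting ends or the component becomes invalid.
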(event Custom|TargetingComponentAdded
  (params (TargetingComponent :type BP%20Targeting%20Component%20Object%20Reference))
  (bind _output_get (Variables|Default|SetTargeting%20Component TargetingComponent))
  (EventDispatchers|BindEventtoNotifyTargetingActive _output_get (delegate Custom|DoTargetLock))
  (CallFunction|DoTargetLock (Variables|/Game/Project4/Blueprints/Component/EventController/Events/Environment/BP_TargetingComponent.BP_TargetingComponent_C|GetTargetingActive _output_get)))

(event Custom|DoTargetLock
  (params (CurrentTargetingActive :type Boolean))
  (Input|SetIgnoreLookInput (Variables|Default|GetOwningPlayerController) CurrentTargetingActive)
  (if CurrentTargetingActive
    (bind _returnvalue (Utilities|Time|SetTimerbyEvent (delegate Custom|DoTargetLockUpdate) (Variables|Default|GetTargetingUpdateTime) true))
    (Variables|Default|SetTargetingTimerHandle _returnvalue)
    (else
      (Utilities|Time|ClearandInvalidateTimerbyHandle (Variables|Default|GetTargetingTimerHandle)))))

(event Custom|DoTargetLockUpdate
  (bind _targeting_component (Variables|Default|GetTargeting%20Component))
  (Utilities|IsValid (Variables|Default|GetTargeting%20Component)
    (:Is%20Valid
      (Pawn|SetControlRotation (Variables|Default|GetOwningPlayerController) (Math|Interpolation|RInterpTo (Pawn|GetControlRotation (Variables|Default|GetOwningPlayerController) :!class /Script/Engine.Controller) (Variables|/Game/Project4/Blueprints/Component/EventController/Events/Environment/BP_TargetingComponent.BP_TargetingComponent_C|GetTargetRotation _targeting_component) (Utilities|Time|GetWorldDeltaSeconds) (Variables|/Game/Project4/Blueprints/Component/EventController/Events/Environment/BP_TargetingComponent.BP_TargetingComponent_C|GetInterp%20Speed _targeting_component))))
    (:Is%20Not%20Valid
      (Utilities|Time|ClearandInvalidateTimerbyHandle (Variables|Default|GetTargetingTimerHandle)))))

(event EventBeginPlay
  (Variables|Default|SetOwningPlayerController (Game|Player|GetOwningPlayerController))
  (EventDispatchers|BindEventtoNotifyTargetingCompAdded (Variables|Default|GetBP_EventController_Component) (delegate Custom|TargetingComponentAdded)))

(fn ConstructionScript)

(fn AsEventControlledCameraManager
  (return self))