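; Base weapon event controller that keeps references to a targeting component and a weapon component.
; On BeginPlay it calls the parent, then binds to the event controller component's notifications for targeting component added, weapon component added and weapon component removed.
; The added handlers store the passed component, and the removed handler clears the weapon reference; the targeting reference has no removal handler.
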(event Custom|OnTargetingComponentAdded
  (params (TargetingComponent :type BP%20Targeting%20Component%20Object%20Reference))
  (Variables|Default|SetTargeting%20Component TargetingComponent))

(event Custom|OnWeaponComponentAdded
  (params (WeaponComponent :type BP%20Weapon%20Component%20Object%20Reference))
  (Variables|Default|SetWeapon%20Component WeaponComponent))

(event Custom|OnWeaponComponentRemoved
  (Variables|Default|SetWeapon%20Component 0))

(event EventBeginPlay
  (|CallParentFunction)
  (EventDispatchers|BindEventtoNotifyTargetingCompAdded (Variables|Default|GetBP_EventController_Component) (delegate Custom|OnTargetingComponentAdded))
  (EventDispatchers|BindEventtoNotifyWeaponComponentAdded (Variables|Default|GetBP_EventController_Component) (delegate Custom|OnWeaponComponentAdded))
  (EventDispatchers|BindEventtoNotifyWeaponComponentRemoved (Variables|Default|GetBP_EventController_Component) (delegate Custom|OnWeaponComponentRemoved)))

(fn ConstructionScript
  (|CallParentFunction))