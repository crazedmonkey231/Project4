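; Actor component that runs one timed game event through the event controller component on its owner.
; On BeginPlay it finds that controller, destroying itself if none exists, unpacks its Event settings and waits the initial delay.
; Each trigger passes the event data to the controller's environment management and a triggered notification.
; Looping events repeat after a delay until the loop count is reached, then the component destroys itself, as one-shot events do immediately.
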(event Custom|DoEvent
  (bind _currenteventcounter (Variables|Default|GetCurrentEventCounter))
  (Utilities|FlowControl|Sequence
    (:then_0
      (Default|DoEnvironmentManagement (Variables|Default|GetEventControllerComponent) (Variables|Default|GetEvent%20Data)))
    (:then_1
      (Default|CallNotifyEventTriggered (Variables|Default|GetEvent%20Data)))
    (:then_2
      (if (Variables|Default|GetLoop)
        (Math|Integer|IncrementInt _currenteventcounter
          (:%20%20
            (if (>= _currenteventcounter (Variables|Default|GetLoop%20Count))
              (Components|DestroyComponent)
              (else
                (Utilities|FlowControl|Delay (Variables|Default|GetLoop%20Event%20Delay))
                (CallFunction|DoEvent)))))
        (else
          (Components|DestroyComponent))))))

(event EventBeginPlay
  (bind _event (Variables|Default|GetEvent))
  (bind (_eventtype _delay _loop _loopcount _loopeventdelay _eventdata) (Utilities|Struct|BreakS_Event _event))
  (Variables|Default|SetOwner (Components|GetOwner))
  (Utilities|FlowControl|Sequence
    (:then_0
      (Utilities|IsValid (Actor|GetComponentbyClass (Variables|Default|GetOwner) (Variables|Default|GetEventControllerClass))
        (:Is%20Valid
          (Variables|Default|SetEventControllerComponent (Actor|GetComponentbyClass (Variables|Default|GetOwner) (Variables|Default|GetEventControllerClass))))
        (:Is%20Not%20Valid
          (Components|DestroyComponent))))
    (:then_1
      (Utilities|FlowControl|Sequence
        (:then_0
          (Variables|Default|SetEvent%20Type _eventtype)
          (Variables|Default|SetDelay _delay)
          (Variables|Default|SetLoop _loop)
          (Variables|Default|SetLoop%20Count _loopcount)
          (Variables|Default|SetLoop%20Event%20Delay _loopeventdelay)
          (Variables|Default|SetEvent%20Data _eventdata))
        (:then_1
          (Utilities|FlowControl|Delay (Variables|Default|GetDelay))
          (CallFunction|DoEvent))))))