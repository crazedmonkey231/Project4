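; Targeting component that, while toggled active, smoothly turns its owning actor toward a target every tick.
; It aims at the target actor's location when valid, otherwise at the stored target location.
; A flag selects whether the owner's X or Y axis points at the target, and RInterpTo eases the rotation.
; The active state has a RepNotify that passes changes on through a notify call.
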(event EventBeginPlay
  (Variables|Default|SetOwner (Components|GetOwner)))

(event EventTick
  (params (DeltaSeconds :type Float%20%28single-precision%29))
  (bind _targetactor (Variables|Default|GetTargetActor))
  (if (Variables|Default|GetTargetingActive)
    (Variables|Default|SetDelta%20Seconds DeltaSeconds)
    (Variables|Default|SetCurrentLocation (Transformation|GetActorLocation (Variables|Default|GetOwner)))
    (Utilities|IsValid _targetactor
      (:Is%20Valid
        (Variables|Default|SetTargetLocation (Transformation|GetActorLocation _targetactor)))
      (:Is%20Not%20Valid
        _))
    (if (Variables|Default|GetUseAxisXorY)
      (Variables|Default|SetTargetRotation (.Rotation (CallFunction|TargettoXZ (Variables|Default|GetCurrentLocation) (Variables|Default|GetTargetLocation))))
      (else
        (Variables|Default|SetTargetRotation (.Rotation (CallFunction|TargettoYZ (Variables|Default|GetCurrentLocation) (Variables|Default|GetTargetLocation))))))
    (Transformation|SetActorRotation (Variables|Default|GetOwner) (CallFunction|DoInterp (Variables|Default|GetTargetRotation)))))

(event EventToggle
  (params (NewToggle :type Boolean))
  (Variables|Default|SetTargetingActive NewToggle))

(fn TargettoXZ
  (params (CurrentLocation :type Vector) (TargetLocation :type Vector))
  (bind _returnvalue (Math|Vector|GetUnitDirection(Vector) CurrentLocation TargetLocation))
  (return _returnvalue (Math|Rotator|MakeRotfromXZ (Math|Vector|GetForwardVector (Math|Rotator|FindLookatRotation CurrentLocation TargetLocation)) _returnvalue)))

(fn TargettoYZ
  (params (CurrentLocation :type Vector) (TargetLocation :type Vector))
  (bind _returnvalue (Math|Vector|GetUnitDirection(Vector) CurrentLocation TargetLocation))
  (return _returnvalue (Class|KismetMathLibrary|MakeRotfromYZ (Math|Vector|GetForwardVector (Math|Rotator|FindLookatRotation CurrentLocation TargetLocation)) _returnvalue)))

(fn DoInterp
  (params (Target :type Rotator))
  (return (Math|Interpolation|RInterpTo (Transformation|GetActorRotation (Variables|Default|GetOwner)) Target (Variables|Default|GetDelta%20Seconds) (Variables|Default|GetInterp%20Speed))))

(fn OnRepTargetingActive
  (Default|CallNotifyTargetingActive (Variables|Default|GetTargetingActive)))