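; Event component that moves its owning actor back and forth between its starting location and an offset set by HoverVector.
; BeginPlay caches both endpoints, and Toggle sets whether hovering is active.
; While active, Tick moves the owner with constant-speed interpolation, flipping direction when it is within tolerance of either endpoint.
; The replication callback for IsHovering passes the new state to a hover-update notify.
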(event EventBeginPlay
  (bind _output_get (Variables|Default|SetOwner (Components|GetOwner)))
  (bind _output_get_2 (Variables|Default|SetStartingLocation (Transformation|GetActorLocation _output_get)))
  (Variables|Default|SetTargetLocation (+ _output_get_2 (Variables|Default|GetHoverVector)))
  (Variables|Default|SetIsForward true))

(event EventToggle
  (params (NewToggle :type Boolean))
  (Variables|Default|SetIsHovering NewToggle))

(event EventTick
  (params (DeltaSeconds :type Float%20%28single-precision%29))
  (if (Variables|Default|GetIsHovering)
    (Variables|Default|SetDelta%20Seconds DeltaSeconds)
    (if (Variables|Default|GetIsForward)
      (Variables|Default|SetInterpLocation (CallFunction|Interpto (Transformation|GetActorLocation (Variables|Default|GetOwner)) (Variables|Default|GetTargetLocation)))
      (else
        (Variables|Default|SetInterpLocation (CallFunction|Interpto (Transformation|GetActorLocation (Variables|Default|GetOwner)) (Variables|Default|GetStartingLocation)))))
    (Transformation|SetActorLocation (Variables|Default|GetOwner) (Variables|Default|GetInterpLocation) false false)
    (Utilities|FlowControl|Sequence
      (:then_0
        (if (Utilities|Operators|EqualEqual (Variables|Default|GetTargetLocation) (Transformation|GetActorLocation (Variables|Default|GetOwner)) (Variables|Default|GetTolerance))
          (Variables|Default|SetIsForward false)))
      (:then_1
        (if (Utilities|Operators|EqualEqual (Variables|Default|GetStartingLocation) (Transformation|GetActorLocation (Variables|Default|GetOwner)) (Variables|Default|GetTolerance))
          (Variables|Default|SetIsForward true))))))

(fn OnRepIsHovering
  (Default|CallNotifyHoverHupdate (Variables|Default|GetIsHovering)))

(fn Interpto
  (params (Current :type Vector) (Target :type Vector))
  (return (Math|Interpolation|VInterptoConstant Current Target (Variables|Default|GetDelta%20Seconds) (Variables|Default|GetInterpSpeed))))