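; Event component that moves its owning actor to a target transform after a delay, then removes itself.
; BeginPlay reads target, interp speed and delay from TransformData; Tick counts up the delay before activating.
; While active, Tick applies TInterpTo to the actor's transform without sweep until it equals the target, then destroys the component.
; Begin, update and end notify calls mark each phase.
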(event EventBeginPlay
  (bind _transformdata (Variables|Default|GetTransformData))
  (bind (_transform _interpspeed _delay) (Utilities|Struct|BreakS_TransformData _transformdata))
  (Variables|Default|SetOwner (Components|GetOwner))
  (Variables|Default|SetTransform _transform)
  (Variables|Default|SetInterp%20Speed _interpspeed)
  (Variables|Default|SetDelay _delay)
  (Variables|Default|SetIsFinishedTransformTo false))

(event EventTick
  (params (DeltaSeconds :type Float%20%28single-precision%29))
  (bind _transform (Variables|Default|GetTransform))
  (bind _owner (Variables|Default|GetOwner))
  (bind _returnvalue (Transformation|GetActorTransform _owner))
  (if (Variables|Default|GetActive)
    (if (Variables|Default|GetIsFinishedTransformTo)
      (Components|DestroyComponent)
      (else
        (Variables|Default|SetNewTransform (Class|KismetMathLibrary|TInterpto _returnvalue _transform DeltaSeconds (Variables|Default|GetInterp%20Speed)))
        (if (== _returnvalue _transform)
          (Variables|Default|SetIsFinishedTransformTo true)
          (Utilities|FlowControl|Sequence
            (:then_0
              (Default|CallNotifyTransformedEnd))
            (:then_1
              (Components|DestroyComponent)))
          (else
            (Utilities|FlowControl|Sequence
              (:then_0
                (Default|CallNotifyTransformUpdate (Variables|Default|GetNewTransform)))
              (:then_1
                (Transformation|SetActorTransform (Variables|Default|GetOwner) (Variables|Default|GetNewTransform))))))))
    (else
      (bind _output_get (Variables|Default|SetDeltaTime (+ (Variables|Default|GetDeltaTime) DeltaSeconds)))
      (if (>= _output_get (Variables|Default|GetDelay))
        (Utilities|FlowControl|Sequence
          (:then_0
            (Default|CallNotifyTransformBegin))
          (:then_1
            (Variables|Default|SetActive true)))))))