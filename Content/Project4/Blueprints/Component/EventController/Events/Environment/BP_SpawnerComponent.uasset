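; Spawner component that, after an initial delay, spawns the actors defined in its ActorSpawnData, owned by the component's owner.
; Each entry's class, or that of its optional override actor, spawns at listed transforms plus those of actors found by class or tag.
; Spawned actors receive optional tags and trigger a notify call.
; DoSpawn re-calls itself after a delay to advance through entries, destroying the component once the index exceeds the list length.
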(event Custom|DoSpawn
  (bind _actors_to_spawn (Variables|Default|GetActors%20to%20Spawn))
  (bind _index (Variables|Default|GetIndex))
  (bind _output (Utilities|Array|Get(acopy) _actors_to_spawn _index))
  (bind (_actortospawn _optionalactoroverride _actortransforms _actortransformsbyclass _actortransformsbytag _optionaltagstoadd) (Utilities|Struct|BreakS_SpawnData _output))
  (if (> _index (Utilities|Array|Length _actors_to_spawn))
    (Components|DestroyComponent)
    (else
      (Variables|Default|SetActorToSpawn _actortospawn)
      (Utilities|FlowControl|Sequence
        (:then_0
          (Utilities|IsValid _optionalactoroverride
            (:Is%20Valid
              (Variables|Default|SetActorToSpawn (Utilities|GetClass _optionalactoroverride)))))
        (:then_1
          (for _array_element (CallFunction|GetTransforms _actortransforms _actortransformsbyclass _actortransformsbytag)
            (bind _returnvalue (Game|SpawnActorfromClass (Variables|Default|GetActorToSpawn) _array_element "Undefined" "MultiplyWithRoot" (Variables|Default|GetOwner) 0))
            (Utilities|FlowControl|Sequence
              (:then_0
                (for _array_element_2 _optionaltagstoadd
                  (Utilities|Array|Add (Variables|/Script/Engine.Actor|GetTags _returnvalue) _array_element_2)))
              (:then_1
                (Utilities|FlowControl|Sequence
                  (:then_0
                    (Default|CallNotifyActorSpawned _returnvalue))
                  (:then_1
                    (Utilities|FlowControl|Delay (Variables|Default|GetDelay%20Between%20Spawn))
                    (Math|Integer|IncrementInt (Variables|Default|GetIndex)
                      (:%20%20
                        (CallFunction|DoSpawn)))))))))))))

(event EventBeginPlay
  (bind _actorspawndata (Variables|Default|GetActorSpawnData))
  (bind (_actorstospawn _delaybetweenspawn _delay) (Utilities|Struct|BreakS_EnvironmentActorSpawnData _actorspawndata))
  (Variables|Default|SetOwner (Components|GetOwner))
  (Variables|Default|SetActors%20to%20Spawn _actorstospawn)
  (Variables|Default|SetDelay%20Between%20Spawn _delaybetweenspawn)
  (Variables|Default|SetDelay _delay)
  (Variables|Default|SetIndex 0)
  (Utilities|FlowControl|Delay (Variables|Default|GetDelay))
  (CallFunction|DoSpawn))

(fn GetTransforms
  (params (ActorTransforms :type Array%20of%20Transforms) (ActorClass :type Array%20of%20Actor%20Class%20References) (ActorTags :type Array%20of%20Names))
  (LocalVariables|SetLocalTransforms ActorTransforms)
  (Utilities|FlowControl|Sequence
    (:then_0
      (for _array_element ActorClass
        (bind _outactors (Actor|GetAllActorsOfClass _array_element))
        (for _array_element_2 _outactors
          (Utilities|Array|Add (LocalVariables|GetLocalTransforms) (Transformation|GetActorTransform _array_element_2)))))
    (:then_1
      (for _array_element_3 ActorTags
        (bind _outactors_2 (Actor|GetAllActorswithTag _array_element_3))
        (for _array_element_4 _outactors_2
          (Utilities|Array|Add (LocalVariables|GetLocalTransforms) (Transformation|GetActorTransform _array_element_4)))))
    (:then_2
      (return (LocalVariables|GetLocalTransforms)))))