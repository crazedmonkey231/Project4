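; BP_HoverComponent is an actor component that moves its owner back and forth between its starting location and an offset by HoverVector.
; A looping timer drives constant-speed interpolation using world delta seconds, flipping direction when either endpoint is within tolerance.
; Toggle switches hovering on or off, and RefreshPositionData re-bases both endpoints on the owner's current location.
; The IsHovering RepNotify calls a hover-update notification with the new state.
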(event Custom|DoHoverUpdate
  (if (Variables|Default|GetIsHovering)
    (if (Variables|Default|GetIsForward)
      (Variables|Default|SetInterpLocation (CallFunction|Interpto (Transformation|GetActorLocation (Variables|Default|GetOwner)) (Variables|Default|GetTargetLocation)))
      (else
        (Variables|Default|SetInterpLocation (CallFunction|Interpto (Transformation|GetActorLocation (Variables|Default|GetOwner)) (Variables|Default|GetStartingLocation)))))
    (Transformation|SetActorLocation (Variables|Default|GetOwner) (Variables|Default|GetInterpLocation) false false)
    (Utilities|FlowControl|Sequence
      (:then_0
        (if (Utilities|Operators|EqualEqual (Variables|Default|GetTargetLocation) (Variables|Default|GetInterpLocation) (Variables|Default|GetTolerance))
          (Variables|Default|SetIsForward false)))
      (:then_1
        (if (Utilities|Operators|EqualEqual (Variables|Default|GetStartingLocation) (Variables|Default|GetInterpLocation) (Variables|Default|GetTolerance))
          (Variables|Default|SetIsForward true))))))

(event Custom|RefreshPositionData
  (bind _output_get (Variables|Default|SetStartingLocation (Transformation|GetActorLocation (Variables|Default|GetOwner))))
  (Variables|Default|SetTargetLocation (+ _output_get (Variables|Default|GetHoverVector))))

(event EventBeginPlay
  (Variables|Default|SetOwner (Components|GetOwner))
  (Variables|Default|SetIsForward true)
  (CallFunction|RefreshPositionData)
  (bind _returnvalue (Utilities|Time|SetTimerbyEvent (delegate Custom|DoHoverUpdate) (Variables|Default|GetHoverUpdateTime) true))
  (Variables|Default|SetHoverUpdateTimerHandle _returnvalue))

(event EventToggle
  (params (NewToggle :type Boolean))
  (Variables|Default|SetIsHovering NewToggle))

(fn OnRepIsHovering
  (Default|CallNotifyHoverHupdate (Variables|Default|GetIsHovering)))

(fn Interpto
  (params (Current :type Vector) (Target :type Vector))
  (return (Math|Interpolation|VInterptoConstant Current Target (Utilities|Time|GetWorldDeltaSeconds) (Variables|Default|GetInterpSpeed))))