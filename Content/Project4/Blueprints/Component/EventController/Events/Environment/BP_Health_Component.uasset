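; Health component that tracks damage taken by its owning actor and destroys that actor when health runs out.
; On BeginPlay it binds to the owner's OnTakeAnyDamage and subtracts incoming damage from Health, clamped between its minimum and maximum.
; Health uses a RepNotify, which broadcasts the NotifyHealthUpdated dispatcher and destroys the owner once the minimum is reached.
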(event Custom|TakeDamage
  (params (DamagedActor :type Actor%20Object%20Reference) (Damage :type Float%20%28single-precision%29) (DamageType :type Damage%20Type%20Object%20Reference) (InstigatedBy :type Controller%20Object%20Reference) (DamageCauser :type Actor%20Object%20Reference))
  (Variables|HealthComponent|SetHealth (Math|Float|Clamp(Float) (- (Variables|HealthComponent|GetHealth) Damage) (Variables|HealthComponent|GetMinHealth) (Variables|HealthComponent|GetMaxHealth))))

(event EventBeginPlay
  (bind _output_get (Variables|HealthComponent|SetOwner (Components|GetOwner)))
  (EventDispatchers|BindEventtoOnTakeAnyDamage _output_get (delegate Custom|TakeDamage)))

(fn OnRepHealth
  (bind _health (Variables|HealthComponent|GetHealth))
  (Default|CallNotifyHealthUpdated _health)
  (if (== _health (Variables|HealthComponent|GetMinHealth))
    (Actor|DestroyActor (Variables|HealthComponent|GetOwner))))