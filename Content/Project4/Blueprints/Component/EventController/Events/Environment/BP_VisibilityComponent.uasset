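; BP_VisibilityComponent is a one-shot environment event component that changes its owning actor's collision and visibility, or removes that actor.
; On BeginPlay it reads VisibilityData and waits for the configured delay before applying the collision and hidden-in-game settings.
; Each change is followed by its own notify call.
; It then destroys either the owner or just itself, depending on the Destroy flag.
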(event EventBeginPlay
  (bind _visibilitydata (Variables|Default|GetVisibilityData))
  (bind (_delay _collision _hidden _destroy) (Utilities|Struct|BreakS_VisibilityData _visibilitydata))
  (Variables|Default|SetOwner (Components|GetOwner))
  (Variables|Default|SetDelay _delay)
  (Variables|Default|SetCollision _collision)
  (Variables|Default|SetHidden _hidden)
  (Variables|Default|SetDestroy _destroy)
  (Utilities|FlowControl|Delay (Variables|Default|GetDelay))
  (Utilities|FlowControl|Sequence
    (:then_0
      (Utilities|FlowControl|Sequence
        (:then_0
          (Collision|SetActorEnableCollision (Variables|Default|GetOwner) (Variables|Default|GetCollision)))
        (:then_1
          (Default|CallNotifyCollisionUpdate (Variables|Default|GetCollision)))))
    (:then_1
      (Utilities|FlowControl|Sequence
        (:then_0
          (Rendering|SetActorHiddenInGame (Variables|Default|GetOwner) (Variables|Default|GetHidden)))
        (:then_1
          (Default|CallNotifyHiddenUpdate (Variables|Default|GetHidden)))))
    (:then_2
      (if (Variables|Default|GetDestroy)
        (Actor|DestroyActor (Variables|Default|GetOwner))
        (else
          (Components|DestroyComponent))))))