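; Targeting component that smoothly turns its owning actor toward a target actor, or the stored target location if the actor is invalid.
; A looping timer started at BeginPlay updates rotation while targeting is toggled on, using RInterpTo with frame delta time rather than the timer interval.
; UseAxisXorY selects an XZ or YZ rotation basis, with both axes fed the direction to the target.
; TargetingActive's OnRep fires a notify dispatcher.
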(event Custom|DoTargetingUpdate
  (bind _targetactor (Variables|Default|GetTargetActor))
  (if (Variables|Default|GetTargetingActive)
    (Variables|Default|SetCurrentLocation (Transformation|GetActorLocation (Variables|Default|GetOwner)))
    (Utilities|IsValid _targetactor
      (:Is%20Valid
        (Variables|Default|SetTargetLocation (Transformation|GetActorLocation _targetactor)))
      (:Is%20Not%20Valid
        _))
    (if (Variables|Default|GetUseAxisXorY)
      (Variables|Default|SetTargetRotation (.Rotation (CallFunction|TargettoXZ (Variables|Default|GetCurrentLocation) (Variables|Default|GetTargetLocation))))
      (else
        (Variables|Default|SetTargetRotation (.Rotation (CallFunction|TargettoYZ (Variables|Default|GetCurrentLocation) (Variables|Default|GetTargetLocation))))))
    (Transformation|SetActorRotation (Variables|Default|GetOwner) (CallFunction|DoInterp (Variables|Default|GetTargetRotation)))))

(event EventBeginPlay
  (Variables|Default|SetOwner (Components|GetOwner))
  (bind _returnvalue (Utilities|Time|SetTimerbyEvent (delegate Custom|DoTargetingUpdate) (Variables|Default|GetTargetingUpdateTime) true))
  (Variables|Default|SetTargetingTimerHandle _returnvalue))

(event EventToggle
  (params (NewToggle :type Boolean))
  (Variables|Default|SetTargetingActive NewToggle))

(fn TargettoXZ
  (params (CurrentLocation :type Vector) (TargetLocation :type Vector))
  (bind _returnvalue (Math|Vector|GetUnitDirection(Vector) CurrentLocation TargetLocation))
  (return _returnvalue (Math|Rotator|MakeRotfromXZ (Math|Vector|GetForwardVector (Math|Rotator|FindLookatRotation CurrentLocation TargetLocation)) _returnvalue)))

(fn TargettoYZ
  (params (CurrentLocation :type Vector) (TargetLocation :type Vector))
  (bind _returnvalue (Math|Vector|GetUnitDirection(Vector) CurrentLocation TargetLocation))
  (return _returnvalue (Class|KismetMathLibrary|MakeRotfromYZ (Math|Vector|GetForwardVector (Math|Rotator|FindLookatRotation CurrentLocation TargetLocation)) _returnvalue)))

(fn DoInterp
  (params (Target :type Rotator))
  (return (Math|Interpolation|RInterpTo (Transformation|GetActorRotation (Variables|Default|GetOwner)) Target (Utilities|Time|GetWorldDeltaSeconds) (Variables|Default|GetInterp%20Speed))))

(fn OnRepTargetingActive
  (Default|CallNotifyTargetingActive (Variables|Default|GetTargetingActive)))