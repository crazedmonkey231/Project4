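; Counter component in the environment event controller folder that keeps a replicated count for other game logic to track.
; Increment and decrement events raise or lower Counter by the One variable.
; The Counter RepNotify broadcasts NotifyCounterUpdated with the new value, so listeners can react to changes without polling.
; AsCounterComponent returns the component itself as a typed accessor.
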(event EventBeginPlay)

(event EventTick
  (params (DeltaSeconds :type Float%20%28single-precision%29)))

(event EventIncrementCounter
  ;[1 1 1] Counter
  (Variables|Default|SetCounter (+ (Variables|Default|GetCounter) (Variables|Default|GetOne))))

(event EventDecrementCounter
  ;[1 1 1] Counter
  (Variables|Default|SetCounter (- (Variables|Default|GetCounter) (Variables|Default|GetOne))))

(fn OnRepCounter
  (Default|CallNotifyCounterUpdated (Variables|Default|GetCounter)))

(fn AsCounterComponent
  (return self))