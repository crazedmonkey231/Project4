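; Toggleable environment sound component that plays an optional 2D sound and an optional 3D sound attached to itself with configurable attenuation.
; Toggle sets the RepNotify IsSoundOn state, whose OnRep passes the new value to CallNotifyIsSoundOnUpdate and refreshes the audio.
; UpdateSounds, also run on BeginPlay, destroys existing audio components and respawns the valid sounds only while the state is on.
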(event EventBeginPlay
  (Variables|Default|SetOwner (Components|GetOwner))
  (CallFunction|UpdateSounds))

(event EventToggle
  (params (NewToggle :type Boolean))
  (Variables|Default|SetIsSoundOn NewToggle))

(fn OnRepIsSoundon
  (Utilities|FlowControl|Sequence
    (:then_0
      (Default|CallNotifyIsSoundonUpdate (Variables|Default|GetIsSoundOn)))
    (:then_1
      (CallFunction|UpdateSounds))))

(fn UpdateSounds
  (Utilities|FlowControl|Sequence
    (:then_0
      (Utilities|FlowControl|Sequence
        (:then_0
          (Utilities|IsValid (Variables|Default|GetSoundComponent2D)
            (:Is%20Valid
              (Components|DestroyComponent (Variables|Default|GetSoundComponent2D)))))
        (:then_1
          (Utilities|IsValid (Variables|Default|GetSoundComponent3D)
            (:Is%20Valid
              (Components|DestroyComponent (Variables|Default|GetSoundComponent3D)))))))
    (:then_1
      (if (Variables|Default|GetIsSoundOn)
        (Utilities|FlowControl|Sequence
          (:then_0
            (Utilities|IsValid (Variables|Default|GetSound2D)
              (:Is%20Valid
                (bind _returnvalue (Audio|SpawnSound2D (Variables|Default|GetSound2D) 1.0 1.0 0.0 0))
                (Variables|Default|SetSoundComponent2D _returnvalue))))
          (:then_1
            (Utilities|IsValid (Variables|Default|GetSound3D)
              (:Is%20Valid
                (bind _returnvalue_2 (Audio|SpawnSoundAttached (Variables|Default|GetSound3D) self "None" "0, 0, 0" "0, 0, 0" "KeepRelativeOffset" true 1.0 1.0 0.0 (Variables|Default|GetSoundAttenuation) 0))
                (Variables|Default|SetSoundComponent3D _returnvalue_2)))))))))