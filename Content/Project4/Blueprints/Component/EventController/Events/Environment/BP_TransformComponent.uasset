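; Actor component in the event controller's environment events that moves its owning actor toward a target transform.
; On BeginPlay it reads target, interpolation speed and start delay from a transform data struct, then starts a looping timer after the delay.
; Each tick of that timer teleports the owner along a TInterpTo step using world delta seconds and broadcasts NotifyTransformUpdate.
; EndPlay clears the timer.
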(event Custom|DoTransformUpdate
  (Variables|Default|SetNewTransform (Class|KismetMathLibrary|TInterpto (Transformation|GetActorTransform (Variables|Default|GetOwner)) (Variables|Default|GetTargetTransform) (Utilities|Time|GetWorldDeltaSeconds) (Variables|Default|GetInterp%20Speed)))
  (Utilities|FlowControl|Sequence
    (:then_0
      (Transformation|SetActorTransform (Variables|Default|GetOwner) (Variables|Default|GetNewTransform) false true))
    (:then_1
      (Default|CallNotifyTransformUpdate (Variables|Default|GetNewTransform)))))

(event EventBeginPlay
  (Variables|Default|SetOwner (Components|GetOwner))
  (CallFunction|SetTransformData (Variables|Default|GetTransformData))
  (Utilities|FlowControl|Delay (Variables|Default|GetDelay))
  (bind _returnvalue (Utilities|Time|SetTimerbyEvent (delegate Custom|DoTransformUpdate) (Variables|Default|GetTransformUpdateTimer) true))
  (Variables|Default|SetTransformTimerHandle _returnvalue))

(event EventEndPlay
  (params (EndPlayReason :type EEndPlayReason%20Enum :default "Destroyed"))
  (Utilities|Time|ClearandInvalidateTimerbyHandle (Variables|Default|GetTransformTimerHandle)))

(fn SetTransformData
  (params (S_TransformData :type S%20Transform%20Data%20Structure%20%28by%20ref%29))
  (bind (_transform _interpspeed _delay) (Utilities|Struct|BreakS_TransformData S_TransformData))
  (Variables|Default|SetTargetTransform _transform)
  (Variables|Default|SetInterp%20Speed _interpspeed)
  (Variables|Default|SetDelay _delay))