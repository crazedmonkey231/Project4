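; Actor component that fires a timed, repeatable interaction through the owner's EventController component, destroying itself if none exists.
; On BeginPlay it unpacks InteractionData into event type, timing, targeting, hover, teleport and projectile defaults, then waits an initial delay.
; DoInteraction messages the controller with itself, broadcasts a notify with the current count, and re-calls itself after a delay until the trigger limit removes the component.
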(event Custom|DoInteraction
  (bind _result (Math|Integer|IncrementInt (Variables|Default|GetCurrentTriggerAmount))
    (:%20%20
      (if (> _result (Variables|Default|GetTrigger%20Amount))
        (Components|DestroyComponent)
        (else
          (Utilities|FlowControl|Sequence
            (:then_0
              (Class|BPIEventControllerComponent|EventControllerInteract(Message) (Variables|Default|GetEventControllerRef) self))
            (:then_1
              (Utilities|FlowControl|Sequence
                (:then_0
                  (Default|CallNotifyInteract (Variables|Default|GetEvent%20Type) (Variables|Default|GetCurrentTriggerAmount)))
                (:then_1
                  (Utilities|FlowControl|Delay (Variables|Default|GetNext%20Trigger%20Delay))
                  (CallFunction|DoInteraction))))))))))

(event EventBeginPlay
  (bind _interactiondata (Variables|Default|GetInteractionData))
  (bind (_eventtype _triggeramount _nexttriggerdelay _delay _interpspeed _defaulttargetingactor _defaulttargetinglocation _defaulthovervector _defaultteleporttoactor _defaultteleporttolocation _defaultprojectileclass) (Utilities|Struct|BreakS_InteractionData _interactiondata))
  (bind _output_get (Variables|Default|SetOwner (Components|GetOwner)))
  (Utilities|IsValid (Actor|GetComponentbyClass _output_get (Variables|Default|GetEventControllerClass))
    (:Is%20Valid
      (Variables|Default|SetEventControllerRef (Actor|GetComponentbyClass _output_get (Variables|Default|GetEventControllerClass)))
      (Utilities|FlowControl|Sequence
        (:then_0
          (Variables|Default|SetEvent%20Type _eventtype)
          (Variables|Default|SetTrigger%20Amount _triggeramount)
          (Variables|Default|SetNext%20Trigger%20Delay _nexttriggerdelay)
          (Variables|Default|SetDelay _delay)
          (Variables|Default|SetInterp%20Speed _interpspeed)
          (Variables|Default|SetDefaultTargetActor _defaulttargetingactor)
          (Variables|Default|SetDefault%20Target%20Location _defaulttargetinglocation)
          (Variables|Default|SetDefault%20Hover%20Vector _defaulthovervector)
          (Variables|Default|SetDefaultTeleportToActor _defaultteleporttoactor)
          (Variables|Default|SetDefaultTeleportToLocation _defaultteleporttolocation)
          (Variables|Default|SetDefault%20Projectile%20Class _defaultprojectileclass))
        (:then_1
          (Variables|Default|SetCurrentTriggerAmount 0)
          (Utilities|FlowControl|Delay (Variables|Default|GetDelay))
          (CallFunction|DoInteraction))))
    (:Is%20Not%20Valid
      (Components|DestroyComponent))))